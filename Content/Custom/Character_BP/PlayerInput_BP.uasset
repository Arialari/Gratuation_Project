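; PlayerInput_BP is the player input pawn, which handles movement and fire controls for a separately spawned craft actor.
; On BeginPlay it spawns a Player_BP at its own transform, stores it as CurrentCharacter and attaches it to itself, keeping world transform.
; Fire presses are forwarded to that craft through FireMessage.
; Forward and right axes move the input pawn along yaw-only directions, carrying the attached craft with it.
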(event `self.ReceiveBeginPlay`
  ;[1 1 1] BeginPlay : 해당 기체 클래스의 인스턴스를 만들고 변수화 시킵니다
  (bind _returnvalue (`|SpawnActorFromClass` "/Game/Custom/Character_BP/Player_BP.Player_BP_C" (`self.GetTransform`) "Undefined" "OverrideRootScale" (`GameplayStatics.GetPlayerPawn` 0) null))
  (bind _output_get (set `self.CurrentCharacter` _returnvalue))
  (`self.K2_AttachToActor` _output_get self "None" "KeepWorld" "KeepWorld" "KeepWorld" true))

(event `InputAction|Fire`
  (params (Key :type "Key Structure"))
  (:`Pressed`
    (message `/Game/Custom/Character_BP/Player_IF.Fire` (`self.CurrentCharacter`))))

(event `InputAxis|MoveForward`
  (params (AxisValue :type "Float (single-precision)"))
  (`self.AddMovementInput` (`KismetMathLibrary.GetForwardVector` (`KismetMathLibrary.MakeRotator` 0.0 0.0 (.yaw (`self.K2_GetActorRotation`)))) AxisValue))

(event `InputAxis|MoveRight`
  (params (AxisValue :type "Float (single-precision)"))
  (`self.AddMovementInput` (`KismetMathLibrary.GetRightVector` (`KismetMathLibrary.MakeRotator` 0.0 0.0 (.yaw (`self.K2_GetActorRotation`)))) AxisValue))

(fn `UserConstructionScript`)