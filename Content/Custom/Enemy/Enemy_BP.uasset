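; Base enemy character for a shooter that faces the player, takes damage and is destroyed at zero HP.
; Start runs a self-rescheduling timer that steps through MovementStruct arrays for direction and speed, which Tick feeds into movement input.
; StartShooting and BulletShooting are empty stubs.
; Freeze stops both timers and rotation, adds a mesh, disables damage and one collision channel response, and drifts the enemy slowly along -X.
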(event `self.ReceiveBeginPlay`
  (`self.BeginPlay`)
  (bind _asmy_player_controller (cast `/Game/Custom/MyPlayerController` (`GameplayStatics.GetPlayerController` 0)))
  (set `self.ProjectileManager` (`/Game/Custom/MyPlayerController.Projectile Manager` _asmy_player_controller)))

(event `self.ReceiveTick`
  (params (DeltaSeconds :type "Float (single-precision)"))
  (`self.TickMovement` DeltaSeconds)
  (if (not (`self.Isfreeze`))
    (`self.LookAtPlayer`)))

(event `self.ReceiveAnyDamage`
  (params (Damage :type "Float (single-precision)") (DamageType :type "DamageType Object Reference") (InstigatedBy :type "Controller Object Reference") (DamageCauser :type "Actor Object Reference"))
  (if (`self.Isfreeze`)
    _
    (else
      _))
  (bind _output_get (set `self.HP` (- (`self.HP`) Damage)))
  (if (<= _output_get 0.0)
    (`self.K2_DestroyActor`)))

(event `/Game/Custom/SkillControl_IF.Freeze`
  (bind _charactermovement (`self.CharacterMovement`))
  ;[1 1 1] Freeze
  (if (not (`self.Isfreeze`))
    (set `self.Isfreeze` true)
    (`self.StopShooting`)
    (`KismetSystemLibrary.K2_ClearAndInvalidateTimerHandle` (`self.MovementTimerHandle`))
    (set `MovementComponent.Velocity` (0.0 0.0 0.0) (`self.CharacterMovement`))
    (set `self.MoveX` -1.0)
    (set `self.MoveY` 0.0)
    (bind _output_get (set `CharacterMovementComponent.MaxWalkSpeed` 100.0 _charactermovement))
    (set `CharacterMovementComponent.MinAnalogWalkSpeed` _output_get _charactermovement)
    (`AddComponent|NODE_AddStaticMeshComponent-0`)
    (set `self.bCanBeDamaged` false)
    (`PrimitiveComponent.SetCollisionResponseToChannel` (`self.SampleMesh`) "ECC_GameTraceChannel1" "ECR_Ignore")))

(fn `BeginPlay`
  (set `self.HP` (`self.MaxHP`)))

(fn `BulletShooting`)

(fn `LookAtPlayer`
  (bind (_returnvalue_roll _returnvalue_pitch _returnvalue_yaw) (`KismetMathLibrary.BreakRotator` (`KismetMathLibrary.FindLookAtRotation` (`self.K2_GetActorLocation`) (`self.K2_GetActorLocation` (`GameplayStatics.GetPlayerCharacter` 0)))))
  (`self.K2_SetActorRotation` (`KismetMathLibrary.MakeRotator` _returnvalue_roll _returnvalue_pitch _returnvalue_yaw)))

(fn `MovementTimer`
  (bind _charactermovement (`self.CharacterMovement`))
  (bind _index (`self.Index`))
  (bind ((`DeltaTime_11_50D0BA08459867E97ED50C90DA558C49` _deltatime) (`MoveX_31_33E3DA7A49A4C37A22F461847D2C5D6A` _movex) (`MoveY_32_0C1DA7E648373353A05F4D8D90DE02A7` _movey) (`MoveSpeed_13_B4A4EFD04A3E63404FEBD7B692270AD4` _movespeed)) (break `/Game/Custom/Enemy/Movement/EnemyMoveStruct` (`self.MovementStruct`)))
  (bind ((`MoveX_31_33E3DA7A49A4C37A22F461847D2C5D6A` _movex_2) (`MoveY_32_0C1DA7E648373353A05F4D8D90DE02A7` _movey_2) (`MoveSpeed_13_B4A4EFD04A3E63404FEBD7B692270AD4` _movespeed_2)) (break `/Game/Custom/Enemy/Movement/EnemyMoveStruct` (`self.MovementStruct`)))
  (bind (_returnvalue_x _returnvalue_y) (`KismetMathLibrary.BreakVector2D` (`KismetMathLibrary.Normal2D` (`KismetMathLibrary.MakeVector2D` (`|GetArrayItem` _movex_2 _index) (`|GetArrayItem` _movey_2 _index)))))
  (set `self.MoveX` _returnvalue_x)
  (set `self.MoveY` _returnvalue_y)
  (bind _output_get (set `CharacterMovementComponent.MaxWalkSpeed` (`|GetArrayItem` _movespeed_2 _index) _charactermovement))
  (set `CharacterMovementComponent.MinAnalogWalkSpeed` _output_get _charactermovement)
  (bind _result (`/Engine/EditorBlueprintResources/StandardMacros.IncrementInt` (`self.Index`))
    (:`  `
      (if (and (< _result (`KismetArrayLibrary.Array_Length` _deltatime)) (< _result (`KismetArrayLibrary.Array_Length` _movex)) (< _result (`KismetArrayLibrary.Array_Length` _movespeed)))
        (bind _returnvalue (`KismetSystemLibrary.K2_SetTimer` null "MovementTimer" (`|GetArrayItem` (`.DeltaTime_11_50D0BA08459867E97ED50C90DA558C49` (break `/Game/Custom/Enemy/Movement/EnemyMoveStruct` (`self.MovementStruct`))) _result)))
        (set `self.MovementTimerHandle` _returnvalue)))))

(fn `Start`
  (`self.StartMoveing`)
  (`self.StartShooting`))

(fn `StartMoveing`
  (set `self.Index` 0)
  (`self.MovementTimer`))

(fn `StartShooting`)

(fn `Stop`
  (`self.StopShooting`)
  (`self.StopMoveing`))

(fn `StopMoveing`
  (`KismetSystemLibrary.K2_ClearAndInvalidateTimerHandle` (`self.MovementTimerHandle`))
  (set `self.MoveX` 0.0)
  (set `self.MoveY` 0.0))

(fn `StopShooting`
  (`KismetSystemLibrary.K2_ClearAndInvalidateTimerHandle` (`self.ShotTimerHandle`)))

(fn `TickMovement`
  (params (A :type "Float (double-precision)"))
  (`self.AddMovementInput` (`KismetMathLibrary.MakeVector` (`self.MoveX`) (`self.MoveY`)) (* A 100.0)))

(fn `UserConstructionScript`
  (`self.SetActorEnableCollision` false))