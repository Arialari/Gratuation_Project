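; Main menu actor that provides character selection with a live, scaled-up preview of the highlighted character.
; On BeginPlay it creates the MainUI widget, removes the player character's Widget component, disables that character's input and spawns Sylphod as the initial preview.
; Left and Right keys cycle MainUI's EnumIndex with wraparound, then ChageChar replaces the preview with the class mapped in EnumToClass, spawned with tick disabled.
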(event `self.ReceiveBeginPlay`
  (bind _asplayer_input_bp (cast `/Game/Custom/Players/PlayerInput_BP` (`GameplayStatics.GetPlayerCharacter` 0)))
  (bind _output_get (set `self.PlayerInputBP` _asplayer_input_bp))
  (bind _returnvalue (`|CreateWidget` "/Game/Custom/UI/mainUI.mainUI_C"))
  (set `/Game/Custom/UI/mainUI.MainMenuBP` self _returnvalue)
  (bind _output_get_2 (set `/Game/Custom/UI/mainUI.PlayerInputBP` _output_get _returnvalue))
  (`ActorComponent.K2_DestroyComponent` (`/Game/Custom/Players/PlayerInput_BP.Widget` _output_get_2))
  (`self.DisableInput` _output_get_2 (`GameplayStatics.GetPlayerController` 0))
  (bind _output_get_3 (set `self.MainUI` _returnvalue))
  (`UserWidget.AddToViewport` _output_get_3 0)
  (bind _returnvalue_2 (`|SpawnActorFromClass` "/Game/Custom/Players/Sylphod/Sylphod.Sylphod_C" (`KismetMathLibrary.MakeTransform` (400.0 -50.0 142.0) (struct) (3.0 3.0 3.0)) "Undefined" "OverrideRootScale" self null))
  (`self.SetActorTickEnabled` _returnvalue_2 false)
  (set `self.CurrentPlayer` _returnvalue_2))

(event `Key|Left`
  (params (Key :type "Key Structure"))
  (bind _mainui (`self.MainUI`))
  (bind _enumindex (`/Game/Custom/UI/mainUI.EnumIndex` _mainui))
  (:`Pressed`
    (if (<= _enumindex (`/Game/Custom/UI/mainUI.MinIndex` _mainui))
      (set `/Game/Custom/UI/mainUI.EnumIndex` (`/Game/Custom/UI/mainUI.MaxIndex` _mainui) _mainui)
      (else
        (set `/Game/Custom/UI/mainUI.EnumIndex` (- _enumindex 1) _mainui)))
    (`self.ChageChar` :!label _label)))

(event `Key|Right`
  (params (Key :type "Key Structure"))
  (bind _mainui (`self.MainUI`))
  (bind _enumindex (`/Game/Custom/UI/mainUI.EnumIndex` _mainui))
  (:`Pressed`
    (if (>= _enumindex (`/Game/Custom/UI/mainUI.MaxIndex` _mainui))
      (set `/Game/Custom/UI/mainUI.EnumIndex` (`/Game/Custom/UI/mainUI.MinIndex` _mainui) _mainui)
      (goto _label)
      (else
        (set `/Game/Custom/UI/mainUI.EnumIndex` (+ _enumindex 1) _mainui)
        (goto _label)))))

(fn `ChageChar`
  (`self.K2_DestroyActor` (`self.CurrentPlayer`))
  (bind _returnvalue (`|SpawnActorFromClass` (`BlueprintMapLibrary.Map_Find` (`self.EnumToClass`) (cast `/Game/Custom/Players/Playable_Character_Name` (`/Game/Custom/UI/mainUI.EnumIndex` (`self.MainUI`)))) (`KismetMathLibrary.MakeTransform` (400.0 -50.0 142.0) (struct) (3.0 3.0 3.0)) "Undefined" "OverrideRootScale" self null))
  (`self.SetActorTickEnabled` _returnvalue false)
  (set `self.CurrentPlayer` _returnvalue))

(fn `UserConstructionScript`)