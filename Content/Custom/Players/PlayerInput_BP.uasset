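; Player character that spawns the craft class matching CharName, attaches it to itself and drives it from input.
; BeginPlay also fills Life and Energy and spawns a projectile pool.
; Movement axes move the character and Slow lowers walk speed, while fire and three skill inputs are forwarded to the craft.
; Damage costs one life, triggering blinking with temporary collision immunity on two channels, or destroys the craft at zero.
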(event `self.ReceiveBeginPlay`
  ;[1 1 1] BeginPlay : 해당 기체 클래스의 인스턴스를 만들고 변수화 시킵니다
  (bind _returnvalue (`|SpawnActorFromClass` (`BlueprintMapLibrary.Map_Find` (`self.Map`) (`self.CharName`)) (`KismetMathLibrary.MakeTransform` (`self.K2_GetActorLocation`)) "AdjustIfPossibleButAlwaysSpawn" "OverrideRootScale" (`GameplayStatics.GetPlayerPawn` 0) null))
  (bind _output_get (set `self.CurrentCharacter` _returnvalue))
  (`self.K2_AttachToActor` _output_get self "None" "KeepWorld" "KeepWorld" "KeepWorld" true)
  (set `self.Energy` (`self.MaxEnergy`))
  (set `self.Life` (`self.MaxLife`))
  (bind _returnvalue_2 (`|SpawnActorFromClass` "/Game/Custom/Projectile/Player_Projectile_Pool.Player_Projectile_Pool_C" (`KismetMathLibrary.MakeTransform` (-2000.0 0.0 142.0)) "Undefined" "OverrideRootScale" self null))
  (set `self.PlayerPool` _returnvalue_2)
  (bind _asmy_player_controller (cast `/Game/Custom/MyPlayerController` (`GameplayStatics.GetPlayerController` 0)))
  (set `self.MyPlayerController` _asmy_player_controller))

(event `self.ReceiveTick`
  (params (DeltaSeconds :type "Float (single-precision)")))

(event `InputAction|Fire`
  (params (Key :type "Key Structure"))
  (:`Pressed`
    (message `/Game/Custom/Players/Player_IF.Fire` (`self.CurrentCharacter`))))

(event `InputAxis|MoveForward`
  (params (AxisValue :type "Float (single-precision)"))
  (`self.AddMovementInput` (`KismetMathLibrary.GetForwardVector` (`KismetMathLibrary.MakeRotator` 0.0 0.0 (.yaw (`self.K2_GetActorRotation`)))) AxisValue))

(event `InputAxis|MoveRight`
  (params (AxisValue :type "Float (single-precision)"))
  (`self.AddMovementInput` (`KismetMathLibrary.GetRightVector` (`KismetMathLibrary.MakeRotator` 0.0 0.0 (.yaw (`self.K2_GetActorRotation`)))) AxisValue))

(event `InputAction|Skill1`
  (params (Key :type "Key Structure"))
  (:`Pressed`
    (message `/Game/Custom/Players/Player_IF.Skill1` (`self.CurrentCharacter`))))

(event `InputAction|Skill2`
  (params (Key :type "Key Structure"))
  (:`Pressed`
    (message `/Game/Custom/Players/Player_IF.Skill2` (`self.CurrentCharacter`))))

(event `InputAction|Skill3`
  (params (Key :type "Key Structure"))
  (:`Pressed`
    (message `/Game/Custom/Players/Player_IF.Skill3` (`self.CurrentCharacter`))))

(event `InputAction|Slow`
  (params (Key :type "Key Structure"))
  (bind _charactermovement (`self.CharacterMovement`))
  (:`Pressed`
    (bind _output_get (set `CharacterMovementComponent.MaxWalkSpeed` (`self.SlowSpeed`) _charactermovement))
    (set `CharacterMovementComponent.MinAnalogWalkSpeed` _output_get _charactermovement))
  (:`Released`
    (bind _output_get_2 (set `CharacterMovementComponent.MaxWalkSpeed` 1000.0 _charactermovement))
    (set `CharacterMovementComponent.MinAnalogWalkSpeed` _output_get_2 _charactermovement)))

(event `self.ReceiveAnyDamage`
  (params (Damage :type "Float (single-precision)") (DamageType :type "DamageType Object Reference") (InstigatedBy :type "Controller Object Reference") (DamageCauser :type "Actor Object Reference"))
  (bind _capsulecomponent (`self.CapsuleComponent`))
  (bind _result (`/Engine/EditorBlueprintResources/StandardMacros.DecrementInt` (`self.Life`))
    (:`  `
      (if (<= _result 0)
        (`self.K2_DestroyActor` (`self.CurrentCharacter`))
        (set `self.bCanBeDamaged` false)
        (else
          (`PrimitiveComponent.SetCollisionResponseToChannel` _capsulecomponent "ECC_GameTraceChannel4" "ECR_Ignore")
          (`PrimitiveComponent.SetCollisionResponseToChannel` _capsulecomponent "ECC_GameTraceChannel5" "ECR_Ignore")
          (set `self.HideCount` (`self.MaxHideCount`))
          (bind _returnvalue (`KismetSystemLibrary.K2_SetTimerDelegate` (delegate `Hide`) 0.1 true))
          (set `self.HideTimerHandle` _returnvalue))))))

(event `Hide`
  (`SceneComponent.ToggleVisibility` (`self.Widget`) true)
  (`SceneComponent.ToggleVisibility` (`Actor.RootComponent` (`self.CurrentCharacter`)) true)
  (bind _output_get (set `self.HideCount` (- (`self.HideCount`) 0.1)))
  (if (not (> _output_get 0.0))
    (`KismetSystemLibrary.K2_ClearAndInvalidateTimerHandle` (`self.HideTimerHandle`))
    (`self.SetActorEnableCollision` true)
    (`SceneComponent.SetVisibility` (`self.RootComponent`) true true)
    (`SceneComponent.SetVisibility` (`self.Widget`) true true)
    (`PrimitiveComponent.SetCollisionProfileName` (`self.CapsuleComponent`) "Player")))

(fn `UserConstructionScript`)